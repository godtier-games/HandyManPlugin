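; BP_BuildingWorldActor is a Geometry Script example actor that procedurally generates a simple building of stacked floor blocks with vertical pillars.
; On mesh rebuild, it extrudes a floor rectangle and repeats it upward once per floor into the target mesh.
; It then places boxes at a temporary rectangle's vertices, sized to the building height plus an offset, and appends them as pillars.
; Temporary compute meshes are released after each rebuild.
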(event Custom|CreateBuildingBlocks_BP
  (params (TargetMesh :type Dynamic%20Mesh%20Object%20Reference))
  (bind _floordimensions (Variables|Default|GetFloorDimensions))
  (bind _returnvalue (DynamicMeshActor|AllocateComputeMesh))
  (bind _returnvalue_2 (Class|GeometryScriptLibraryMeshPrimitiveFunctions|AppendRectangleXY :TargetMesh _returnvalue :DimensionX (.x _floordimensions) :DimensionY (.y _floordimensions) :Debug 0))
  (bind _returnvalue_3 (Class|GeometryScriptLibraryMeshModelingFunctions|ApplyMeshLinearExtrudeFaces :TargetMesh _returnvalue_2 :Options (Utilities|Struct|MakeGeometryScriptMeshLinearExtrudeOptions (Variables|Default|GetBP_FloorHeight) "FixedDirection") :Debug 0))
  (bind _returnvalue_4 (Class|GeometryScriptLibraryMeshBasicEditFunctions|AppendMeshRepeated TargetMesh _returnvalue_3 (Math|Transform|MakeTransform (Math|Vector|MakeVector 0.0 0.0 (Variables|Default|GetBP_FloorHeight))) (Variables|Default|GetBP_NumberOfFloors) false false "(CombineMode=EnableAllMatching)" 0))
  (Variables|Default|SetBP_BuildingBlocks _returnvalue_4))

(event Custom|CreatePillars_BP
  (params (TargetMesh :type Dynamic%20Mesh%20Object%20Reference))
  (bind _bp_pillarthickness (Variables|Default|GetBP_PillarThickness))
  (bind _floordimensions (Variables|Default|GetFloorDimensions))
  (bind _returnvalue (DynamicMeshActor|AllocateComputeMesh))
  (bind _returnvalue_2 (Class|GeometryScriptLibraryMeshPrimitiveFunctions|AppendRectangleXY :TargetMesh _returnvalue :DimensionX (.x _floordimensions) :DimensionY (.y _floordimensions) :Debug 0))
  (bind _positionlist (GeometryScript|MeshQueries|GetAllVertexPositions _returnvalue_2))
  (bind _returnvalue_3 (DynamicMeshActor|AllocateComputeMesh))
  (for _index (range 0 (- (Class|GeometryScriptLibraryListUtilityFunctions|GetVectorListLength _positionlist) 1))
    (bind _returnvalue_4 (Class|GeometryScriptLibraryMeshPrimitiveFunctions|AppendBox :TargetMesh _returnvalue_3 :Transform (Math|Conversions|ToTransform(Vector) (.ReturnValue (Class|GeometryScriptLibraryListUtilityFunctions|GetVectorListItem _positionlist _index))) :DimensionX _bp_pillarthickness :DimensionY _bp_pillarthickness :DimensionZ (+ (* (Variables|Default|GetBP_FloorHeight) (Variables|Default|GetBP_NumberOfFloors)) (Variables|Default|GetBP_PillarOffset)) :Debug 0))
    (Variables|Default|SetBP_Pillars _returnvalue_4))
  (GeometryScript|MeshEdits|AppendMesh :TargetMesh TargetMesh :AppendMesh (Variables|Default|GetBP_Pillars) :AppendOptions "(CombineMode=EnableAllMatching)" :Debug 0))

(event Events|EventOnRebuildGeneratedMesh
  (params (TargetMesh :type Dynamic%20Mesh%20Object%20Reference))
  (Utilities|FlowControl|Sequence
    (:then_0
      (CallFunction|CreateBuildingBlocksBP TargetMesh))
    (:then_1
      (CallFunction|CreatePillarsBP (Variables|Default|GetBP_BuildingBlocks)))
    (:then_2
      (DynamicMeshActor|ReleaseAllComputeMeshes))))

(fn ConstructionScript)