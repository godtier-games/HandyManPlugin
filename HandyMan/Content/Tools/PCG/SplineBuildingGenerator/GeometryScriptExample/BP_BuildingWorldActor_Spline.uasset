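; Geometry Script generated-mesh actor that experiments with building procedural building blocks along a spline.
; On rebuild it extrudes a floor-sized rectangle once per sampled spline frame, using location plus forward vector as direction, appends each result, then releases compute meshes.
; A pillar event places boxes at rectangle corners, but its only call is disconnected, as is an older stacked-floor extrusion.
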(event Custom|CreateBuildingBlocks_BP
  (params (TargetMesh :type Dynamic%20Mesh%20Object%20Reference))
  (bind _floordimensions (Variables|Default|GetFloorDimensions))
  (bind _returnvalue (DynamicMeshActor|AllocateComputeMesh))
  (bind _returnvalue_2 (Class|GeometryScriptLibraryMeshPrimitiveFunctions|AppendRectangleXY :TargetMesh _returnvalue :Transform (Math|Transform|MakeTransform "0, 0, 0" "90.000000,0.000000,0.000000") :DimensionX (.x _floordimensions) :DimensionY (.y _floordimensions) :Debug 0))
  (bind _frames (Class|GeometryScriptLibraryPolyPathFunctions|SampleSplinetoTransforms :Spline (Variables|Default|GetSpline) :SamplingOptions (Utilities|Struct|MakeGeometryScriptSplineSamplingOptions 10 1.0)))
  (for _array_element _frames
    (bind _returnvalue_3 (Class|GeometryScriptLibraryMeshModelingFunctions|ApplyMeshLinearExtrudeFaces :TargetMesh _returnvalue_2 :Options (Utilities|Struct|MakeGeometryScriptMeshLinearExtrudeOptions 1.0 "FixedDirection" (+ (.Location (Math|Transform|BreakTransform _array_element)) (Math|Vector|GetForwardVector (.Rotation (Math|Transform|BreakTransform _array_element))))) :Debug 0))
    (GeometryScript|MeshEdits|AppendMesh :TargetMesh TargetMesh :AppendMesh _returnvalue_3 :AppendOptions "(CombineMode=EnableAllMatching)" :Debug 0)))

(event Custom|CreatePillars_BP
  (params (TargetMesh :type Dynamic%20Mesh%20Object%20Reference))
  (bind _bp_pillarthickness (Variables|Default|GetBP_PillarThickness))
  (bind _floordimensions (Variables|Default|GetFloorDimensions))
  (bind _returnvalue (DynamicMeshActor|AllocateComputeMesh))
  (bind _returnvalue_2 (Class|GeometryScriptLibraryMeshPrimitiveFunctions|AppendRectangleXY :TargetMesh _returnvalue :DimensionX (.x _floordimensions) :DimensionY (.y _floordimensions) :Debug 0))
  (bind _positionlist (GeometryScript|MeshQueries|GetAllVertexPositions _returnvalue_2))
  (bind _returnvalue_3 (DynamicMeshActor|AllocateComputeMesh))
  (for _index (range 0 (- (Class|GeometryScriptLibraryListUtilityFunctions|GetVectorListLength _positionlist) 1))
    (bind _returnvalue_4 (Class|GeometryScriptLibraryMeshPrimitiveFunctions|AppendBox :TargetMesh _returnvalue_3 :Transform (Math|Conversions|ToTransform(Vector) (.ReturnValue (Class|GeometryScriptLibraryListUtilityFunctions|GetVectorListItem _positionlist _index))) :DimensionX _bp_pillarthickness :DimensionY _bp_pillarthickness :DimensionZ (+ (* (Variables|Default|GetBP_FloorHeight) (Variables|Default|GetBP_NumberOfFloors)) (Variables|Default|GetBP_PillarOffset)) :Debug 0))
    (Variables|Default|SetBP_Pillars _returnvalue_4))
  (GeometryScript|MeshEdits|AppendMesh :TargetMesh TargetMesh :AppendMesh (Variables|Default|GetBP_Pillars) :AppendOptions "(CombineMode=EnableAllMatching)" :Debug 0))

(event Events|EventOnRebuildGeneratedMesh
  (params (TargetMesh :type Dynamic%20Mesh%20Object%20Reference))
  (CallFunction|CreateBuildingBlocksBP TargetMesh)
  (DynamicMeshActor|ReleaseAllComputeMeshes))

(fn ConstructionScript)