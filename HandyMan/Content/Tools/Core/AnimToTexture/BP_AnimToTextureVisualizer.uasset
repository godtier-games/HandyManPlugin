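; Visualizer Blueprint for AnimToTexture that previews baked animation on a single HISM instance added by the construction script.
; Each Tick derives CurrentFrame from real time at 30 fps, wrapped using the first Data animation's frame bounds (divisor is start minus end plus one).
; It writes CurrentFrame, PreviousFrame and Alpha into per-instance custom data, though only CurrentFrame is computed here.
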(event EventBeginPlay)

(event Collision|EventActorBeginOverlap
  (params (OtherActor :type Actor%20Object%20Reference)))

(event EventTick
  (params (DeltaSeconds :type Float%20%28single-precision%29))
  (CallFunction|CalculateCurrentFrame)
  (Components|InstancedStaticMesh|SetCustomDataValue (Variables|Default|GetHISM) 0 0 (Variables|Default|GetCurrentFrame) true)
  (Components|InstancedStaticMesh|SetCustomDataValue (Variables|Default|GetHISM) 0 1 (Variables|Default|GetPreviousFrame) true)
  (Components|InstancedStaticMesh|SetCustomDataValue (Variables|Default|GetHISM) 0 2 (Variables|Default|GetAlpha) true))

(fn ConstructionScript
  (Components|InstancedStaticMesh|AddInstance (Variables|Default|GetHISM) (Math|Transform|MakeTransform "0, 0, 0") false))

(fn CalculateCurrentFrame
  (bind _data (Variables|Default|GetData))
  (bind _animations (Variables|/Script/AnimToTexture.AnimToTextureDataAsset|GetAnimations _data))
  (bind _output (Utilities|Array|Get(acopy) _animations))
  (Variables|Default|SetCurrentFrame (+ (.Remainder (Math|Float|Division(WholeandRemainder) (* (Utilities|Time|GetRealTimeSeconds) 3e+01 1.0) (Math|Conversions|ToFloat(Integer) (+ (- (.startframe _output) (.endframe _output)) 1)))) (.startframe _output))))